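; BP_InteractionTest is a lesson test actor with a sphere that gives visible and audible feedback when interacted with.
; The construction script creates a dynamic material instance on the sphere and stores it as DMI.
; The Interact event sets that instance's Color parameter to a random opaque color, then spawns an asteroid explosion particle effect and plays an explosion sound at the actor's root location.
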(event `Interact`
  (bind _returnvalue (`SceneComponent.K2_GetComponentLocation` (`self.DefaultSceneRoot`)))
  (`MaterialInstanceDynamic.SetVectorParameterValue` (`self.DMI`) "Color" (make `LinearColor` (`KismetMathLibrary.RandomFloatInRange` 0.0 1.0) (`KismetMathLibrary.RandomFloatInRange` 0.0 1.0) (`KismetMathLibrary.RandomFloatInRange` 0.0 1.0) 1.0))
  (`GameplayStatics.SpawnEmitterAtLocation` "/Game/Effects/Particles/Explosion/P_AsteroidExplosion.P_AsteroidExplosion" _returnvalue)
  (`GameplayStatics.PlaySoundAtLocation` "/Game/Audio/SoundWaves/Effect/SW_Explosion_1.SW_Explosion_1" _returnvalue))

(fn `UserConstructionScript`
  (bind _returnvalue (`PrimitiveComponent.CreateDynamicMaterialInstance` (`self.Sphere`) 0 null))
  (set `self.DMI` _returnvalue))