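; Lesson 3 player pawn that aims a reticle and interacts with objects by tracing from the VR camera.
; BeginPlay adds a camera control component, and Tick rotates a mesh to the aim rotation with an offset.
; Tick also line-traces forward to place the reticle at the hit or at maximum trace distance.
; The Act input repeats the trace, calls InteractMessage on the hit actor and prints its name and the result.
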(event `InputAction|Act`
  (params (Key :type "Key Structure" :default "AnyKey"))
  (:`Pressed`
    ;[1 1 1] Ray Trace function
    (bind (_location _forward_vector) (`/Game/Blueprints/Utility/LayoutVRUtilityFunctions.Get Player VR Camera Properties`))
    (bind (_outhit _returnvalue) (`KismetSystemLibrary.LineTraceSingle` _location (+ _location (* _forward_vector (`self.TraceDistance`))) "TraceTypeQuery1"))
    (if _returnvalue
      (bind (_bblockinghit _binitialoverlap _time _location_2 _impactpoint _normal _impactnormal _physmat _hitactor) (`GameplayStatics.BreakHitResult` _outhit))
      (`KismetSystemLibrary.PrintString` (`KismetStringLibrary.Concat_StrStr` (`KismetSystemLibrary.GetDisplayName` _hitactor) " is hit!"))
      (bind _score (message `/Game/Lessons/Lesson3/BPI_Interaction.Interact` _hitactor))
      (`KismetSystemLibrary.PrintString` (`KismetStringLibrary.Conv_IntToString` _score) true true (struct :`R` 1.0 :`B` 0.121763 :`A` 1.0)))))

(event `self.ReceiveBeginPlay`
  (`AddComponent|NODE_AddBPC_CameraControl-0`) ; Bind pawn to user input
)

(event `self.ReceiveTick`
  (params (DeltaSeconds :type "Float (single-precision)"))
  (bind _reticle (`self.Reticle`))
  (`SceneComponent.K2_SetWorldRotation` (`self.StaticMesh`) (`KismetMathLibrary.MakeRotator` (+ (.roll (`self.GetBaseAimRotation`)) -90.0) (+ (.pitch (`self.GetBaseAimRotation`)) -90.0) (.yaw (`self.GetBaseAimRotation`))) false false)
  ;[1 1 1] Ray Trace function
  (bind (_location _forward_vector) (`/Game/Blueprints/Utility/LayoutVRUtilityFunctions.Get Player VR Camera Properties`))
  (bind _returnvalue (+ _location (* _forward_vector (`self.TraceDistance`))))
  (bind (_outhit _returnvalue_2) (`KismetSystemLibrary.LineTraceSingle` :`Start` _location :`End` _returnvalue :`TraceChannel` "TraceTypeQuery1" :`DrawTime` 0.05))
  (if _returnvalue_2
    (`SceneComponent.K2_SetWorldLocation` _reticle (`.Location` (`GameplayStatics.BreakHitResult` _outhit)) false false)
    (else
      (`SceneComponent.K2_SetWorldLocation` _reticle _returnvalue false false))))

(fn `UserConstructionScript`)