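; BP_Explodable is a homework actor that explodes once when another actor overlaps it.
; On BeginPlay it switches off its radial force and sets HasExploded for two seconds, so early overlaps cannot trigger it.
; The first overlap after that spawns an asteroid explosion particle, activates the radial force, turns the mesh material black and plays audio.
; The HasExploded flag then blocks repeat explosions, and the actor stays in the level.
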(event `self.ReceiveBeginPlay`
  (set `self.hasExploded` true)
  (`ActorComponent.Deactivate` (`self.RadialForce`))
  (`KismetSystemLibrary.Delay` 2.0)
  (set `self.hasExploded` false))

(event `self.ReceiveActorBeginOverlap`
  (params (OtherActor :type "Actor Object Reference"))
  (if (not (`self.hasExploded`))
    (`GameplayStatics.SpawnEmitterAtLocation` "/Game/Effects/Particles/Explosion/P_AsteroidExplosion2.P_AsteroidExplosion2" (`SceneComponent.K2_GetComponentLocation` (`self.Explodable`)))
    (set `self.hasExploded` true)
    (`ActorComponent.Activate` (`self.RadialForce`) false)
    (`PrimitiveComponent.SetMaterial` (`self.Explodable`) 0 "/Game/Materials/Solids/Dual_Color/MI_Black_Black.MI_Black_Black")
    (`AudioComponent.Play` (`self.Audio`) 0.0)))

(fn `UserConstructionScript`)