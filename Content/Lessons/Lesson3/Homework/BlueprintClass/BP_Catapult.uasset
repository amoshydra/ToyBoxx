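; Catapult actor that fires one second after BeginPlay and again on its launch event, playing audio as the arm swings.
; A timeline pitches PointOfRotation, and a retriggerable delay on its updates starts the retract timeline three seconds after the swing ends.
; IsLoading blocks the load event from launch until retraction begins; otherwise that event spawns a BP_Explodable at AmmoSpawnPoint.
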(event `self.ReceiveBeginPlay`
  (`KismetSystemLibrary.Delay` 1.0)
  (`AudioComponent.Play` (`self.Audio`) 0.0 :!label _label)
  (set `self.isLoading` true)
  (bind (_direction _track_launch) (`Timeline|Timeline_0` :!via `PlayFromStart`)
    (:`Update`
      (`SceneComponent.K2_SetRelativeRotation` (`self.PointOfRotation`) (`KismetMathLibrary.MakeRotator` (.roll (`SceneComponent.RelativeRotation` (`self.PointOfRotation`))) _track_launch (.yaw (`SceneComponent.RelativeRotation` (`self.PointOfRotation`)))) true false)
      (`KismetSystemLibrary.RetriggerableDelay` 3.0)
      (bind (_direction_2 _track_retract) (`Timeline|Timeline_1` :!via `PlayFromStart`)
        (:`Update`
          (`SceneComponent.K2_SetRelativeRotation` (`self.PointOfRotation`) (`KismetMathLibrary.MakeRotator` (.roll (`SceneComponent.RelativeRotation` (`self.PointOfRotation`))) _track_retract (.yaw (`SceneComponent.RelativeRotation` (`self.PointOfRotation`)))) true false)
          (set `self.isLoading` false))))))

(event `/Game/Lessons/Lesson3/Homework/BlueprintClass/BPI/BPI_Single_CatapultLaunch.Single-CatapultLaunch`
  (goto _label))

(event `Load Ammunation_Event`
  (if (not (`self.isLoading`))
    (`|SpawnActorFromClass` "/Game/Lessons/Lesson3/Homework/BlueprintClass/BP_Explodable.BP_Explodable_C" (`KismetMathLibrary.MakeTransform` (`SceneComponent.K2_GetComponentLocation` (`self.AmmoSpawnPoint`))) "Undefined" "OverrideRootScale")))

(fn `UserConstructionScript`)