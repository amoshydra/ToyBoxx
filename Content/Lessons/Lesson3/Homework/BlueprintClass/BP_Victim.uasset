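; BP_Victim is a lesson homework Blueprint for a victim that walks its static mesh along until it tips over and counts as dead.
; Each Tick nudges the mesh by a fixed relative offset, mostly along negative Y, without sweep or delta-time scaling.
; Once the mesh's absolute relative pitch reaches the tilt threshold, IsDead latches and movement stops for good.
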(event `self.ReceiveBeginPlay`
  (set `self.isDead` false))

(event `self.ReceiveTick`
  (params (DeltaSeconds :type "Float (single-precision)"))
  (if (`self.isDead`)
    _
    (elif (>= (`KismetMathLibrary.Abs` (.pitch (`SceneComponent.RelativeRotation` (`self.StaticMesh`)))) 50.0)
      (set `self.isDead` true)
      (else
        (`SceneComponent.K2_AddRelativeLocation` (`self.StaticMesh`) (0.0 -1.0 1e-06) false false)))))

(fn `UserConstructionScript`)