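; BP_InteractionPlayer0 is a lesson player Blueprint that interacts with objects through a camera-forward line trace on left mouse click.
; A hit prints the actor's name, and a hit BP_InteractionTest receives Interact() and spawns a neon explosion at its location.
; BeginPlay adds camera control and a billboard component.
; Tick aligns the static mesh to aim rotation with an offset and moves the billboard to the last trace hit location.
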(event `Key|LeftMouseButton`
  (params (Key :type "Key Structure" :default "AnyKey"))
  (:`Pressed`
    (bind (_location _forward_vector) (`/Game/Blueprints/Utility/LayoutVRUtilityFunctions.Get Player VR Camera Properties`))
    (bind (_outhit _returnvalue) (`KismetSystemLibrary.LineTraceSingle` :`Start` _location :`End` (+ _location (* _forward_vector (`self.TraceDistance`))) :`TraceChannel` "TraceTypeQuery1" :`DrawDebugType` "ForDuration"))
    (if _returnvalue
      (bind (_bblockinghit _binitialoverlap _time _location_2 _impactpoint _normal _impactnormal _physmat _hitactor) (`GameplayStatics.BreakHitResult` _outhit))
      (`KismetSystemLibrary.PrintString` (`KismetStringLibrary.Concat_StrStr` (`KismetSystemLibrary.GetDisplayName` _hitactor) " is hit!"))
      (bind _asbp_interaction_test (cast `/Game/Lessons/Lesson3/BP_InteractionTest` _hitactor))
      (`/Game/Lessons/Lesson3/BP_InteractionTest.Interact` _asbp_interaction_test)
      (`GameplayStatics.SpawnEmitterAtLocation` "/Game/Effects/Particles/Explosion/P_NeonExplosion.P_NeonExplosion" (`self.K2_GetActorLocation` _hitactor)))))

(event `self.ReceiveBeginPlay`
  (`AddComponent|BPC Camera Control_0`)
  (bind _returnvalue (`AddComponent|MaterialBillboardComponent_1`)))

(event `self.ReceiveTick`
  (params (DeltaSeconds :type "Float (single-precision)"))
  (`SceneComponent.K2_SetWorldRotation` (`self.StaticMesh`) (`KismetMathLibrary.MakeRotator` (+ (.roll (`self.GetBaseAimRotation`)) -90.0) (+ (.pitch (`self.GetBaseAimRotation`)) -90.0) (.yaw (`self.GetBaseAimRotation`))) false false)
  (`SceneComponent.K2_SetWorldLocation` (stale `self.ReceiveBeginPlay` _returnvalue) (`.Location` (`GameplayStatics.BreakHitResult` (stale `Key|LeftMouseButton` _outhit))) false false))

(fn `UserConstructionScript`)