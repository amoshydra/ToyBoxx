(event `self.ReceiveBeginPlay`
  (bind _returnvalue (`GameplayStatics.GetPlayerController` 0))
  (`KismetSystemLibrary.Delay` 6.0)
  (bind (_direction _lookdown) (`Timeline|Timeline_0`)
    (:`Update`
      (`Controller.SetControlRotation` _returnvalue (`KismetMathLibrary.MakeRotator` (.roll (`Controller.GetControlRotation` _returnvalue)) _lookdown (.yaw (`Controller.GetControlRotation` _returnvalue)))))))

(event `InputAxis|MoveForward`
  (params (AxisValue :type "Float (single-precision)"))
  ;[1 1 1] Navigation
  (`self.AddMovementInput` (`self.GetActorForwardVector`) AxisValue))

(event `InputAxis|Turn`
  (params (AxisValue :type "Float (single-precision)"))
  ;[1 1 1] Camera
  (`self.AddControllerYawInput` AxisValue))

(event `InputAxis|LookUp`
  (params (AxisValue :type "Float (single-precision)"))
  ;[1 1 1] Camera
  (`self.AddControllerPitchInput` AxisValue))

(event `InputAxis|MoveRight`
  (params (AxisValue :type "Float (single-precision)"))
  ;[1 1 1] Navigation
  (`self.AddMovementInput` (`self.GetActorRightVector`) AxisValue))

(event `InputAction|Jump`
  (params (Key :type "Key Structure" :default "AnyKey"))
  ;[1 1 1] Movement
  (:`Pressed`
    (`self.Jump`))
  (:`Released`
    (`self.StopJumping`)))

(event `Key|LeftControl`
  (params (Key :type "Key Structure" :default "AnyKey"))
  (:`Pressed`
    (`self.Crouch`))
  (:`Released`
    (`self.UnCrouch`)))

(event `self.ReceiveTick`
  (params (DeltaSeconds :type "Float (single-precision)"))
  ;[1 1 1] Ray Trace function
  (bind (_location _forward_vector) (`/Game/Blueprints/Utility/LayoutVRUtilityFunctions.Get Player VR Camera Properties`))
  (bind (_outhit _returnvalue) (`KismetSystemLibrary.LineTraceSingle` :`Start` _location :`End` (+ _location (* _forward_vector 100000.0)) :`TraceChannel` "TraceTypeQuery1" :`DrawTime` 1.0))
  (if _returnvalue
    (bind (_bblockinghit _binitialoverlap _time _location_2 _impactpoint _normal _impactnormal _physmat _hitactor) (`GameplayStatics.BreakHitResult` _outhit))
    (message `/Game/Lessons/Lesson3/Homework/BlueprintClass/BPI/BPI_Gaze_Hover.Gaze_Hover` _hitactor)
    (`SceneComponent.K2_SetWorldLocation` (`self.Reticle`) _location_2 false false)))

(event `InputAction|GazeSelect`
  (params (Key :type "Key Structure" :default "AnyKey"))
  (:`Pressed`
    ;[1 1 1] Ray Trace function
    (bind (_location _forward_vector) (`/Game/Blueprints/Utility/LayoutVRUtilityFunctions.Get Player VR Camera Properties`))
    (bind (_outhit _returnvalue) (`KismetSystemLibrary.LineTraceSingle` :`Start` _location :`End` (+ _location (* _forward_vector 100000.0)) :`TraceChannel` "TraceTypeQuery1" :`DrawTime` 1.0))
    (if _returnvalue
      (bind (_bblockinghit _binitialoverlap _time _location_2 _impactpoint _normal _impactnormal _physmat _hitactor _hitcomponent) (`GameplayStatics.BreakHitResult` _outhit))
      (message `/Game/Lessons/Lesson3/Homework/BlueprintClass/BPI/BPI_Gaze_Click.Gaze_Click` _hitactor null)
      (`KismetSystemLibrary.PrintString` (`KismetSystemLibrary.GetDisplayName` _hitcomponent)))))

(fn `UserConstructionScript`)