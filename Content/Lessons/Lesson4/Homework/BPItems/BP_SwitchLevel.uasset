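; BP_SwitchLevel is a switch actor that toggles when it receives a GazeClick event.
; Each click flips IsActivated and snaps the AxisOfRotation component between its rest and rotated positions.
; Switching on also finds the first BP_SuperPlane in the world and calls its ActivateDoorEvent, while switching off only resets the rotation and state.
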(event `self.ReceiveBeginPlay`
  (set `self.isActivated` false))

(event `/Game/Lessons/Lesson3/Homework/BlueprintClass/BPI/BPI_Gaze_Click.Gaze_Click`
  (params (HitActor :type "Actor Object Reference"))
  (bind _axisofrotation (`self.AxisOfRotation`))
  (if (`self.isActivated`)
    (`SceneComponent.K2_SetRelativeRotation` _axisofrotation (struct) false false)
    (set `self.isActivated` false)
    (else
      (`SceneComponent.K2_SetRelativeRotation` _axisofrotation (struct :`Roll` 120.0) false false)
      (set `self.isActivated` true)
      (bind _outactors (`GameplayStatics.GetAllActorsOfClass` "/Game/Lessons/Lesson4/Homework/BPItems/BP_SuperPlane.BP_SuperPlane_C"))
      (`/Game/Lessons/Lesson4/Homework/BPItems/BP_SuperPlane.ActivateDoor_Event` (`KismetArrayLibrary.Array_Get` _outactors)))))

(fn `UserConstructionScript`)