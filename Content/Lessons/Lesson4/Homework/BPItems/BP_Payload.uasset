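; BP_Payload is a lesson homework item that arms on actor overlap and can then be detonated by a gaze click.
; After a short retriggerable delay, the first overlap plays a beep, sets HasEnabled and prints an activation message.
; Ten seconds later it sets IsReady and toggles two point lights in a repeating delay loop.
; GazeClick checks only HasEnabled before spawning a neon explosion and replaying the beep.
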(event `/Game/Lessons/Lesson3/Homework/BlueprintClass/BPI/BPI_Gaze_Click.Gaze_Click`
  (params (HitActor :type "Actor Object Reference"))
  (if (`self.hasEnabled`)
    (`GameplayStatics.SpawnEmitterAtLocation` "/Game/Effects/Particles/Explosion/P_NeonExplosion.P_NeonExplosion" (`SceneComponent.K2_GetComponentLocation` (`self.DefaultSceneRoot`)))
    (`AudioComponent.Play` (`self.clean-modem-beep_Cue`) 0.0)))

(event `self.ReceiveActorBeginOverlap`
  (params (OtherActor :type "Actor Object Reference"))
  (`KismetSystemLibrary.RetriggerableDelay` 0.2)
  (if (not (`self.hasEnabled`))
    (`AudioComponent.Play` (`self.clean-modem-beep_Cue`) 0.0)
    (set `self.hasEnabled` true)
    (`KismetSystemLibrary.PrintString` "Payload activated")
    (`KismetSystemLibrary.Delay` 10.0)
    (set `self.isReady` true)
    (`KismetSystemLibrary.Delay` 1.5 :!label _label)
    (`SceneComponent.ToggleVisibility` (`self.PointLight1`) false)
    (`SceneComponent.ToggleVisibility` (`self.PointLight`) false)
    (if (`self.hasEnabled`)
      (goto _label))))

(fn `UserConstructionScript`)