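; BP_SuperPlane is a lesson homework actor that lights up and swings open a gate-like part shortly after play begins.
; After a short delay on BeginPlay, it sets all its point light components to the activated color, then plays a timeline.
; The timeline's Decreasing track drives the roll of AxisOfRotation to open the gate.
; A per-light interval delay is left disconnected, so all lights change at once.
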(event `self.ReceiveBeginPlay`
  (bind _axisofrotation (`self.AxisOfRotation`))
  (`KismetSystemLibrary.Delay` 2.0)
  (for _array_element (`self.K2_GetComponentsByClass` "/Script/Engine.PointLightComponent")
    (`LightComponent.SetLightColor` _array_element (`self.LightActivatedColor`) true))
  (bind (_direction _decreasing) (`Timeline|Timeline_0`)
    (:`Update`
      ;[1 1 1] OpenGate
      (`SceneComponent.K2_SetRelativeRotation` _axisofrotation (`KismetMathLibrary.MakeRotator` (* _decreasing 62.0) (.pitch (`SceneComponent.RelativeRotation` _axisofrotation)) (.yaw (`SceneComponent.RelativeRotation` _axisofrotation))) false false))))

(fn `UserConstructionScript`)