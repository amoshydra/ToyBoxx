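; Movable cloud actor that drifts through the level along world X and loops back once it travels too far.
; While ShouldCloudMove is set, Tick offsets it in negative X at a speed re-randomized every frame, scaled by delta time.
; Dropping below LifeDistance triggers a debug print and a forward jump that wraps it around.
; The SkyStop event clears the flag to halt the cloud.
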(event `self.ReceiveBeginPlay`)

(event `/Game/Lessons/Lesson4/Homework/BPItems/BP_SkyStop.SkyStop`
  (set `self.shouldCloudMove` false))

(event `self.ReceiveTick`
  (params (DeltaSeconds :type "Float (single-precision)"))
  (if (`self.shouldCloudMove`)
    (`self.K2_AddActorWorldOffset` (`KismetMathLibrary.MakeVector` (* DeltaSeconds (`KismetMathLibrary.RandomFloatInRange` -6000.0 -4000.0))))
    (if (> (`self.LifeDistance`) (.x (`SceneComponent.K2_GetComponentLocation` (`self.DefaultSceneRoot`))))
      (`KismetSystemLibrary.PrintString` (`KismetStringLibrary.Conv_DoubleToString` 0.0) true true (struct :`G` 0.66 :`B` 1.0 :`A` 1.0) 1.0)
      (`self.K2_AddActorWorldOffset` (`KismetMathLibrary.MakeVector` (+ (- 0.0 (`self.LifeDistance`)) 20000.0))))))

(fn `UserConstructionScript`)