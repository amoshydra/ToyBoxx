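; BP_Water is a homework-lesson water actor that moves up and down to imitate waves.
; Each Tick it adds a small Z offset to its current location, using the sine of game time scaled by WaveMagnitude.
; Game time is truncated to whole seconds, so the step changes once per second.
; The offset accumulates without delta-time scaling, so motion depends on frame rate.
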(event `self.ReceiveTick`
  (params (DeltaSeconds :type "Float (single-precision)"))
  (`self.K2_SetActorLocation` (+ (`self.K2_GetActorLocation`) (* (0.0 0.0 0.1) (* (- (`KismetMathLibrary.Sin` (`KismetMathLibrary.Conv_IntToDouble` (`KismetMathLibrary.FTrunc` (`KismetSystemLibrary.GetGameTimeInSeconds`)))) 0.0) (`self.WaveMagnitude`))))))

(fn `UserConstructionScript`)