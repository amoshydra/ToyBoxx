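; BP_NPCKnockable_Player is a lesson homework actor that serves as the player's view target and gets knocked over on overlap.
; On BeginPlay it takes over the first controller's view and sets control rotation from the skeletal mesh's rotation, then Tick copies control rotation onto the camera's relative rotation.
; An overlap reveals a text render, enables mesh physics, then after a short delay enables gravity and plays a drum sound.
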(event EventBeginPlay
  (bind _self self)
  (bind _skeletalmesh (Variables|Default|GetSkeletalMesh _self))
  (bind _returnvalue (Transformation|GetWorldRotation _skeletalmesh))
  (bind (_roll _pitch _yaw) (Math|Rotator|BreakRotator _returnvalue))
  (Game|Player|SetViewTargetwithBlend (Game|GetPlayerController 0) self 0.0 "VTBlend_Linear" 0.0 false)
  (Pawn|SetControlRotation (Game|GetPlayerController 0) (Math|Rotator|MakeRotator _roll _pitch (stale _result))))

(event Collision|EventActorBeginOverlap
  (params (OtherActor :type Actor%20Object%20Reference))
  (bind _skeletalmesh (Variables|Default|GetSkeletalMesh))
  (Rendering|SetVisibility (Variables|Default|GetTextRender) true false)
  (Physics|SetSimulatePhysics _skeletalmesh true)
  (Utilities|FlowControl|Delay 0.2)
  (Physics|SetEnableGravity _skeletalmesh true)
  (Audio|PlaySoundatLocation "/Game/Audio/SoundWaves/Drum/SW_PacificIslandDrum.SW_PacificIslandDrum" (Transformation|GetWorldLocation _skeletalmesh)))

(event EventTick
  (params (DeltaSeconds :type Float%20%28single-precision%29))
  (Transformation|SetRelativeRotation (Variables|Default|GetCamera) (Pawn|GetControlRotation (Game|GetPlayerController 0) :!class /Script/Engine.Controller) false false))

(fn ConstructionScript)