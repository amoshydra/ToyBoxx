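; BP_Popping_Balloon is a lesson actor for a balloon that floats upward and pops when something overlaps it.
; Each tick it moves straight up with a swept world offset scaled by delta time and a Speed variable.
; An overlap plays an explosion sound and particle effect at its location, then destroys it.
; If nothing pops it, it destroys itself after a short delay from BeginPlay.
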(event `self.ReceiveBeginPlay`
  (`KismetSystemLibrary.Delay` 6.0)
  (`self.K2_DestroyActor`))

(event `self.ReceiveActorBeginOverlap`
  (params (OtherActor :type "Actor Object Reference"))
  (bind _returnvalue (`self.K2_GetActorLocation`))
  (`GameplayStatics.SpawnSoundAtLocation` "/Game/Audio/SoundWaves/Effect/SW_Explosion_2.SW_Explosion_2" _returnvalue)
  (`GameplayStatics.SpawnEmitterAtLocation` "/Game/Effects/Particles/Explosion/P_AsteroidExplosion.P_AsteroidExplosion" _returnvalue)
  (`self.K2_DestroyActor`))

(event `self.ReceiveTick`
  (params (DeltaSeconds :type "Float (single-precision)"))
  (`self.K2_AddActorWorldOffset` (* (`KismetMathLibrary.MakeVector` 0.0 0.0 (* DeltaSeconds 75.0)) (* (0.0 0.0 1.0) (`self.Speed`))) true))

(fn `UserConstructionScript`)